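; Fire storm weapon action that circles a particle effect around the owning character.
; DoAction plays the action only when the owner's IState interface reports idle, switching it to the action state.
; Beginning the action attaches the emitter to Box at a random start angle, and Tick orbits Box around the owner while the effect exists.
; Ending waits for Timer, destroys the effect and returns the owner to idle.
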(event `self.ReceiveBeginPlay`
  ;[1 1 1] BeginPlay
  (`parent.ReceiveBeginPlay`)
  (`PrimitiveComponent.SetCollisionEnabled` (`self.Box`) "NoCollision"))

(event `self.DoAction`
  (bind _ownercharacter (`self.OwnerCharacter`))
  ;[1 1 1] DoAction
  (`parent.DoAction`)
  (if (`KismetSystemLibrary.DoesImplementInterface` _ownercharacter "/Game/Interfaces/IState.IState_C")
    (bind _result (message `/Game/Interfaces/IState.IsState_Idle` _ownercharacter))
    (if _result
      (message `/Game/Interfaces/IState.SetState_DoAction` _ownercharacter)
      (`self.PlayAction` 0))))

(event `self.Begin_DoAction`
  (bind (_effect _location _rotation _scale) (`self.GetActionEffect` 0))
  (`parent.Begin_DoAction`)
  (bind _returnvalue (`GameplayStatics.SpawnEmitterAttached` _effect (`self.Box`) "None" _location _rotation _scale))
  (set `self.Paticle` _returnvalue)
  (set `self.Angle` (`KismetMathLibrary.RandomFloatInRange` 0.0 360.0)))

(event `self.End_DoAction`
  (bind _ownercharacter (`self.OwnerCharacter`))
  (`parent.End_DoAction`)
  (`KismetSystemLibrary.Delay` (`self.Timer`))
  (`ActorComponent.K2_DestroyComponent` (`self.Paticle`))
  (if (`KismetSystemLibrary.DoesImplementInterface` _ownercharacter "/Game/Interfaces/IState.IState_C")
    (message `/Game/Interfaces/IState.SetState_Idle` _ownercharacter)))

(event `self.ReceiveTick`
  (params (DeltaSeconds :type "Float (single-precision)"))
  (`self.Paticle`
    (:`then`
      (`|ExecutionSequence`
        (:`then_0`
          (bind _output_get (set `self.Angle` (+ (* (`self.Speed`) (`GameplayStatics.GetWorldDeltaSeconds`)) (`self.Angle`))))
          (if (`KismetMathLibrary.NearlyEqual_FloatFloat` _output_get 360.0)
            (set `self.Angle` 0.0)))
        (:`then_1`
          (`SceneComponent.K2_SetWorldLocation` (`self.Box`) (+ (`KismetMathLibrary.RotateAngleAxis` (`KismetMathLibrary.MakeVector` (`self.Distance`) 0.0) (`self.Angle`) (0.0 0.0 1.0)) (`self.K2_GetActorLocation` (`self.OwnerCharacter`))) false false))))
    (:`else`)))

(fn `GetCursorLocationAndRotation`
  (returns (HitResult :type Boolean) (HitResultImpactPoint :type "Vector Structure") (HitResultImpacttNormal :type "Rotator Structure"))
  (return false (0.0 0.0 0.0)))

(fn `UserConstructionScript`
  (`parent.UserConstructionScript`))