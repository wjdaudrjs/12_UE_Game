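; BP_Warp is a weapon that teleports its owning character to the point under the mouse cursor.
; While equipped by a Player-tagged owner, Tick aligns a decal to the WorldStatic surface hit by a cursor trace.
; DoAction caches that hit and, if the owner's IState is idle, plays the action.
; BeginDoAction spawns an effect on the mesh, and EndDoAction moves the owner to the cached point and restores its state.
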(event `self.ReceiveBeginPlay`
  ;[1 1 1] BeginPlay
  (`parent.ReceiveBeginPlay`)
  (`SceneComponent.SetVisibility` (`self.Decal`) false false))

(event `self.UnEquip`
  ;[1 1 1] Unequip
  (`parent.UnEquip`)
  (`SceneComponent.SetVisibility` (`self.Decal`) false false))

(event `self.ReceiveTick`
  (params (DeltaSeconds :type "Float (single-precision)"))
  (bind (_hitresult _hitresultimpactpoint _hitresultimpactnormal) (`self.GetCursorLocationandRotation`))
  (bind _decal (`self.Decal`))
  ;[1 1 1] Tick
  (if (`self.GetEquipped`)
    (if (`self.IsVisibleCursor`)
      (if _hitresult
        (`SceneComponent.SetVisibility` _decal true false)
        (`SceneComponent.K2_SetWorldLocationAndRotation` (`self.Decal`) _hitresultimpactpoint _hitresultimpactnormal false false)
        (else
          (`SceneComponent.SetVisibility` _decal false false))))))

(event `self.DoAction`
  (bind (_hitresult _hitresultimpactpoint) (`self.GetCursorLocationandRotation`))
  (bind _ownercharacter (`self.OwnerCharacter`))
  ;[1 1 1] DoAction
  (`parent.DoAction`)
  (set `self.Possible` _hitresult)
  (set `self.ImpactPoint` _hitresultimpactpoint)
  (if _hitresult
    (if (`KismetSystemLibrary.DoesImplementInterface` _ownercharacter "/Game/Interfaces/IState.IState_C")
      (bind _result (message `/Game/Interfaces/IState.IsState_Idle` _ownercharacter))
      (if _result
        (message `/Game/Interfaces/IState.SetState_DoAction` _ownercharacter)
        (`self.PlayAction` 0)))))

(event `self.Begin_DoAction`
  (bind (_effect _location _rotation _scale) (`self.GetActionEffect` 0))
  ;[1 1 1] BeginDoAction
  (`parent.Begin_DoAction`)
  (if (`self.Possible`)
    (`GameplayStatics.SpawnEmitterAttached` _effect (`Character.Mesh` (`self.OwnerCharacter`)) "None" _location _rotation _scale)))

(event `self.End_DoAction`
  (bind _ownercharacter (`self.OwnerCharacter`))
  ;[1 1 1] EndDoAction
  (`parent.End_DoAction`)
  (if (`self.Possible`)
    (`self.K2_SetActorLocation` _ownercharacter (`self.ImpactPoint`) false false)
    (message `/Game/Interfaces/IState.SetState_Idle` _ownercharacter)
    (message `/Game/Interfaces/IWeapon.SetWeapon_Move` _ownercharacter)))

(fn `GetCursorLocationandRotation`
  (returns (HitResult :type Boolean) (HitResultImpactPoint :type "Vector Structure") (HitResultImpactNormal :type "Rotator Structure"))
  (bind (_hitresult _returnvalue) (`PlayerController.GetHitResultUnderCursorForObjects` (`GameplayStatics.GetPlayerController` 0) (`|MakeArray` "ObjectTypeQuery1" :!type "EObjectTypeQuery Enum") false))
  (return _returnvalue (`.ImpactPoint` (`GameplayStatics.BreakHitResult` _hitresult)) (`KismetMathLibrary.Conv_VectorToRotator` (`.ImpactNormal` (`GameplayStatics.BreakHitResult` _hitresult)))))

(fn `IsVisibleCursor`
  (returns (Result :type Boolean))
  (if (`self.ActorHasTag` (`self.OwnerCharacter`) "Player")
    (return true)
    (else
      (return false))))

(fn `UserConstructionScript`
  (`parent.UserConstructionScript`))