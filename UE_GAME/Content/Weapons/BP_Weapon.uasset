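; Base weapon Blueprint that tracks equipped state, attaches to its owner character's mesh and plays data-driven action montages.
; On BeginPlay it caches the ActionTable rows and owner, then filters those rows by WeaponType to look up actions.
; PlayAction plays the indexed montage and sends move or stop messages through the owner's IWeapon interface.
; BeginEquip and the DoAction functions are empty, apparently hooks for child weapons.
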(event `self.ReceiveBeginPlay`
  (`|ExecutionSequence`
    (:`then_0`
      (bind _actiontable (`self.ActionTable`)
        (:`then`
          (bind _outrownames (`DataTableFunctionLibrary.GetDataTableRowNames` _actiontable))
          (for _array_element _outrownames
            (bind _returnvalue (`|GetDataTableRow` (`self.ActionTable`) _array_element)
              (:`then`
                (`KismetArrayLibrary.Array_Add` (`self.ActionDatas`) _returnvalue)))))
        (:`else`)))
    (:`then_1`
      (bind _ascharacter (cast `Character` (`self.GetOwner`)))
      (set `self.OwnerCharacter` _ascharacter))))

(fn `AttachToOwnerCharacter`
  (params (InSocketName :type Name))
  (`self.K2_AttachToComponent` (`Character.Mesh` (`self.OwnerCharacter`)) InSocketName "KeepRelative" "KeepRelative" "KeepRelative"))

(fn `Begin_DoAction`)

(fn `Begin_Equip`)

(fn `DoAction`)

(fn `End_DoAction`)

(fn `End_Equip`
  (set `self.Equipped` true))

(fn `GetActionCanMove`
  (params (InIndex :type Integer))
  (returns (canMove :type Boolean))
  (bind (_output_type _output_montage _output_playratio _output_canmove) (break `/Game/Structures/FAction` (`|GetArrayItem` (`self.GetActions`) InIndex)))
  (return _output_canmove))

(fn `GetActions`
  (returns (OutActions :type "Array of /Game/Structures/FAction Structure"))
  (locals (Actions :type "Array of /Game/Structures/FAction Structure"))
  (for _array_element (`self.ActionDatas`)
    (if (`|EnumEquality` (`.Type_26_05C0CE804D2B1B430E7CBB9988AAFAC5` (break `/Game/Structures/FAction` _array_element)) (`self.WeaponType`))
      (`KismetArrayLibrary.Array_Add` (`local.Actions`) _array_element)))
  (return (`local.Actions`)))

(fn `GetActionStop`
  (params (InIndex :type Integer))
  (returns (Stop :type "Float (double-precision)"))
  (bind (_output_type _output_montage _output_playratio _output_canmove _output_damage _output_stop) (break `/Game/Structures/FAction` (`|GetArrayItem` (`self.GetActions`) InIndex)))
  (return _output_stop))

(fn `GetEquipped`
  (returns (Result :type Boolean))
  (return (`self.Equipped`)))

(fn `IsExistAction`
  (returns (OutResult :type Boolean))
  (for _array_element (`self.ActionDatas`)
    (if (`|EnumEquality` (break `/Game/Structures/FAction` _array_element) (`self.WeaponType`))
      (return true)))
  (return false))

(fn `PlayAction`
  (params (InIndex :type Integer))
  (bind _ownercharacter (`self.OwnerCharacter`))
  (bind (_output_type _output_montage _output_playratio) (break `/Game/Structures/FAction` (`|GetArrayItem` (`self.GetActions`) (`local.InIndex`))))
  (`Character.PlayAnimMontage` (`self.OwnerCharacter`) _output_montage _output_playratio "None")
  (if (`KismetSystemLibrary.DoesImplementInterface` _ownercharacter "/Game/InterFaces/IWeapon.IWeapon_C")
    (if (`self.GetActionCanMove` (`local.InIndex`))
      (message `/Game/InterFaces/IWeapon.SetWeapon_Move` _ownercharacter)
      (else
        (message `/Game/InterFaces/IWeapon.SetWeapon_Stop` _ownercharacter)))))

(fn `UnEquip`
  (set `self.Equipped` false))

(fn `UserConstructionScript`)