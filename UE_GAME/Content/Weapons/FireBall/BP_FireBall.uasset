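; Fireball weapon attached to its owning character, showing its particle effect only while equipped.
; Its action runs from idle state via IState, spawning a projectile at the FireBall socket that damages characters, bursts and is destroyed on overlap.
; Holding the skill zooms the camera through timelines and toggles the IWeapon crosshair.
; While that crosshair shows, Tick traces a horizontally flattened aim line for pawns, turning it red on a hit.
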(event `self.ReceiveBeginPlay`
  ;[1 1 1] BeginPlay
  (`parent.ReceiveBeginPlay`)
  (`self.AttachToOwnerCharacter` "None")
  (`SceneComponent.SetVisibility` (`self.ParticleSystem`) false false))

(event `self.End_Equip`
  ;[1 1 1] EndEquip
  (`parent.End_Equip`)
  (`SceneComponent.SetVisibility` (`self.ParticleSystem`) true false))

(event `self.UnEquip`
  ;[1 1 1] UnEquip
  (`parent.UnEquip`)
  (`SceneComponent.SetVisibility` (`self.ParticleSystem`) false false))

(event `self.DoAction`
  (bind _ownercharacter (`self.OwnerCharacter`))
  ;[1 1 1] DoAction
  (`parent.DoAction`)
  (if (`KismetSystemLibrary.DoesImplementInterface` _ownercharacter "/Game/Interfaces/IState.IState_C")
    (bind _result (message `/Game/Interfaces/IState.IsState_Idle` _ownercharacter))
    (if _result
      (message `/Game/Interfaces/IState.SetState_DoAction` _ownercharacter)
      (`self.PlayAction` 0))))

(event `self.End_DoAction`
  (bind _ownercharacter (`self.OwnerCharacter`))
  ;[1 1 1] EndDoAction
  (`parent.End_DoAction`)
  (if (`KismetSystemLibrary.DoesImplementInterface` _ownercharacter "/Game/Interfaces/IState.IState_C")
    (message `/Game/Interfaces/IState.SetState_Idle` _ownercharacter)))

(event `OnBeginOverlap`
  (params (Causer :type "Actor Object Reference") (OtherActor :type "Actor Object Reference"))
  (bind (_effect _location _rotation _scale) (`self.GetActionEffect` 0))
  ;[1 1 1] Begin Overlap
  (bind _ascharacter (cast `Character` OtherActor)
    (:`then`
      (`self.SendDamage` _ascharacter (`self.GetActionDamage` 0)))
    (:`CastFailed`
      _))
  (`GameplayStatics.SpawnEmitterAtLocation` _effect (+ _location (`self.K2_GetActorLocation` Causer)) _rotation _scale)
  (`self.K2_DestroyActor` Causer))

(event `self.Begin_DoAction`
  (bind _ownercharacter (`self.OwnerCharacter`))
  ;[1 1 1] BeginDoAction
  (`parent.Begin_DoAction`)
  (bind _returnvalue (`|SpawnActorFromClass` (`self.GetActionProjecttile` 0) (`KismetMathLibrary.MakeTransform` (`SceneComponent.GetSocketLocation` (`Character.Mesh` _ownercharacter) "FireBall") (`Pawn.GetControlRotation` _ownercharacter)) "Undefined" "OverrideRootScale" self null))
  (add `/Game/Weapons/FireBall/BP_Projecttile.OnBeginOverlap` _returnvalue (`|CreateDelegate` :!event `OnBeginOverlap`)))

(event `self.Pressed_DoSkill`
  (bind _ownercharacter (`self.OwnerCharacter`))
  (bind _returnvalue (`self.GetComponentByClass` (`self.OwnerCharacter`) "/Script/Engine.SpringArmComponent"))
  (bind _returnvalue_2 (`self.GetComponentByClass` (`self.OwnerCharacter`) "/Script/Engine.CameraComponent"))
  ;[1 1 1] PressDoSkill
  (`parent.Pressed_DoSkill`)
  (if (`self.Use Camera Controller`)
    (set `SpringArmComponent.TargetArmLength` 100.0 _returnvalue)
    (set `SpringArmComponent.SocketOffset` (0.0 30.0 0.0) _returnvalue)
    (bind (_direction _fov) (`Timeline|Zoom` :!via `PlayFromStart`)
      (:`Update`
        (`CameraComponent.SetFieldOfView` _returnvalue_2 _fov)
        (`SceneComponent.K2_SetRelativeLocation` _returnvalue_2 (0.0 0.0 0.0) false false))
      (:`Finished`
        (if (`KismetSystemLibrary.DoesImplementInterface` _ownercharacter "/Game/Interfaces/IWeapon.IWeapon_C")
          (bind _result (message `/Game/Interfaces/IWeapon.GetWeapon_CrossHair` _ownercharacter))
          (`/Engine/EditorBlueprintResources/StandardMacros.IsValid` _result
            (:`Is Valid`
              (`Widget.SetVisibility` _result "Visible"))))))))

(event `self.Release_DoSkill`
  (bind _ownercharacter (`self.OwnerCharacter`))
  (bind _returnvalue (`self.GetComponentByClass` (`self.OwnerCharacter`) "/Script/Engine.SpringArmComponent"))
  (bind _returnvalue_2 (`self.GetComponentByClass` (`self.OwnerCharacter`) "/Script/Engine.CameraComponent"))
  ;[1 1 1] RelaseDoSkill
  (`parent.Release_DoSkill`)
  (if (`self.Use Camera Controller`)
    (set `SpringArmComponent.TargetArmLength` 280.0 _returnvalue)
    (set `SpringArmComponent.SocketOffset` (0.0 0.0 0.0) _returnvalue)
    (bind (_direction _fov) (`Timeline|타임라인_0` :`NewTime` 0.0 :!via `ReverseFromEnd`)
      (:`Update`
        (`CameraComponent.SetFieldOfView` _returnvalue_2 _fov)
        (`SceneComponent.K2_SetRelativeLocation` _returnvalue_2 (-16.0 0.0 33.0) false false))
      (:`Finished`
        (if (`KismetSystemLibrary.DoesImplementInterface` _ownercharacter "/Game/Interfaces/IWeapon.IWeapon_C")
          (bind _result (message `/Game/Interfaces/IWeapon.GetWeapon_CrossHair` _ownercharacter))
          (`/Engine/EditorBlueprintResources/StandardMacros.IsValid` _result
            (:`Is Valid`
              (`Widget.SetVisibility` _result "Hidden"))))))))

(event `self.ReceiveTick`
  (params (DeltaSeconds :type "Float (single-precision)"))
  (bind _ownercharacter (`self.OwnerCharacter`))
  (bind _ownercharacter_2 (`self.OwnerCharacter`))
  (bind _returnvalue (`self.GetComponentByClass` _ownercharacter "/Script/Engine.CameraComponent"))
  (bind _returnvalue_2 (`SceneComponent.K2_GetComponentLocation` _returnvalue))
  (if (`self.GetEquipped`)
    (if (`KismetSystemLibrary.DoesImplementInterface` _ownercharacter_2 "/Game/Interfaces/IWeapon.IWeapon_C")
      (bind _result (message `/Game/Interfaces/IWeapon.GetWeapon_CrossHair` _ownercharacter_2))
      (`/Engine/EditorBlueprintResources/StandardMacros.IsValid` _result
        (:`Is Valid`
          (if (`|EnumEquality` (`Widget.GetVisibility` _result) "Visible")
            (`/Engine/EditorBlueprintResources/StandardMacros.IsValid` _returnvalue
              (:`Is Valid`
                (bind (_outhit _returnvalue_3) (`KismetSystemLibrary.LineTraceSingleForObjects` _returnvalue_2 (+ _returnvalue_2 (* (`KismetMathLibrary.Vector_Normal2D` (`KismetMathLibrary.GetForwardVector` (`Pawn.GetControlRotation` _ownercharacter))) (`self.TraceDistance`))) (`|MakeArray` "ObjectTypeQuery3" :!type "EObjectTypeQuery Enum") false (`|MakeArray` (`self.OwnerCharacter`) :!type "Actor Object Reference")))
                (if _returnvalue_3
                  (`/Game/UserInterface/WB_CrossHair.ChangeColor_Red` _result)
                  (else
                    (`/Game/UserInterface/WB_CrossHair.ChangeColor_White` _result)))))))))))

(fn `Use Camera Controller`
  (returns (Result :type Boolean))
  (return (and (`KismetSystemLibrary.IsValid` (`self.GetComponentByClass` (`self.OwnerCharacter`) "/Script/Engine.SpringArmComponent")) (`KismetSystemLibrary.IsValid` (`self.GetComponentByClass` (`self.OwnerCharacter`) "/Script/Engine.CameraComponent")))))

(fn `UserConstructionScript`
  (`parent.UserConstructionScript`))